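; Door actor Blueprint that swings open and closed by 90 degrees of yaw.
; Each Lookingat event flips the IsOpen state and adds a positive or negative relative rotation to the SMDoor component.
; The rotation is applied instantly, with no timeline or interpolation, and its angle is set on BeginPlay.
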(event EventBeginPlay
  (Variables|Default|SetRotation 9e+01))

(event EventLookingat
  (bind _rotation (Variables|Default|GetRotation))
  ;[1 1 1] Toggle switch
  (bind _output_get (Variables|Default|SetisOpen (not (Variables|Default|GetisOpen))))
  (if _output_get
    (Transformation|AddRelativeRotation (Variables|Default|GetSM_Door) (Math|Rotator|MakeRotator 0.0 0.0 _rotation) false false)
    (else
      (Transformation|AddRelativeRotation (Variables|Default|GetSM_Door) (Math|Rotator|MakeRotator 0.0 0.0 (* -1 _rotation)) false false))))

(fn ConstructionScript)