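; Ceiling fan actor whose two point lights can be switched on and off.
; BeginPlay sets both lights to a fixed intensity.
; The Lookingat event flips an IsOff flag, then either zeroes both lights or restores that intensity.
; The graphs contain no blade rotation logic, and the construction script is empty.
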(event EventBeginPlay
  (Variables|Default|SetIntensity 3e+03)
  (Rendering|Components|Light|SetIntensity (Variables|Default|GetPointLight) (Variables|Default|GetIntensity)))

(event EventLookingat
  ;[1 1 1] Toggle switch
  (bind _output_get (Variables|Default|SetisOff (not (Variables|Default|GetisOff))))
  (if _output_get
    (Rendering|Components|Light|SetIntensity (Variables|Default|GetPointLight) 0.0)
    (else
      (Rendering|Components|Light|SetIntensity (Variables|Default|GetPointLight) (Variables|Default|GetIntensity)))))

(fn ConstructionScript)