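; BP_Tile is a floor segment for a side-scrolling runner that extends the track and may carry an obstacle.
; The player overlapping SpawnTrigger asks the game mode for another tile, any DespawnTrigger overlap destroys this one, and AttachPoint provides an attach transform.
; The construction script may add a child-actor obstacle at a random low, mid or high point.
; A countdown shared through RunnerInstance spaces out probability rolls, resetting even when a roll fails.
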(event OnComponentBeginOverlap(DespawnTrigger)
  (params (OverlappedComponent :type Primitive%20Component%20Object%20Reference) (OtherActor :type Actor%20Object%20Reference) (OtherComp :type Primitive%20Component%20Object%20Reference) (OtherBodyIndex :type Integer) (bFromSweep :type Boolean) (SweepResult :type Hit%20Result%20Structure%20%28by%20ref%29))
  (Actor|DestroyActor))

(event OnComponentBeginOverlap(SpawnTrigger)
  (params (OverlappedComponent :type Primitive%20Component%20Object%20Reference) (OtherActor :type Actor%20Object%20Reference) (OtherComp :type Primitive%20Component%20Object%20Reference) (OtherBodyIndex :type Integer) (bFromSweep :type Boolean) (SweepResult :type Hit%20Result%20Structure%20%28by%20ref%29))
  (Utilities|Casting|CastToSideScrollerCharacter OtherActor)
  (bind _asrunner_side_scroller_game_mode (Utilities|Casting|CastToRunnerSideScrollerGameMode (Game|GetGameMode)))
  (Default|AddFloorTile _asrunner_side_scroller_game_mode))

(fn ConstructionScript
  (CallFunction|SetSpawnPoints)
  (CallFunction|SpawnObstacle))

(fn GetAttachTransform
  (return (Transformation|GetWorldTransform (Variables|Default|GetAttach%20point))))

(fn SetSpawnPoints
  (Variables|Default|SetSpawnPoints (Utilities|Array|MakeArray (Transformation|GetRelativeTransform (Variables|Default|GetSpawnPointLow)) (Transformation|GetRelativeTransform (Variables|Default|GetSpawnPointMid)) (Transformation|GetRelativeTransform (Variables|Default|GetSpawnPointHigh)))))

(fn SpawnObstacle
  (bind _spawnpoints (Variables|Default|GetSpawnPoints))
  (bind _canspawnobstacle (CallFunction|IsObstacleSpawnable))
  (if _canspawnobstacle
    (AddComponent|AddChildActorComponent false (Utilities|Array|Get(acopy) _spawnpoints (Math|Random|RandomIntegerinRange 0 (Utilities|Array|LastIndex _spawnpoints))))))

(fn IsObstacleSpawnable
  ;[1 1 1] Wait for tiles logic
  (bind _waitfortiles (CallFunction|GetWaitforTiles))
  ;[1 1 1] Decrement after executing
  (bind _result (Math|Integer|DecrementInt _waitfortiles)
    (:%20%20
      (CallFunction|SetWaitforTiles _result)
      (Utilities|FlowControl|Sequence
        (:then_0
          ;[1 1 1] amount of empty spaces between obstacles
          (if (<= _waitfortiles 0)
            (CallFunction|SetWaitforTiles (Variables|Default|GetInter-SpawnGracePeriod))))
        (:then_1
          ;[0.8642 0.3444 1] return wait for tiles and random value
          (return (and (<= _waitfortiles 0) (< (Math|Random|RandomFloat) (Variables|Default|GetSpawnProbablility)))))))))

(fn GetWaitforTiles
  (bind _asrunner_instance (Utilities|Casting|CastToRunnerInstance (Game|GetGameInstance)))
  (return (Variables|/Game/Assets/Blueprints/RunnerInstance.RunnerInstance_C|GetWaitForTiles _asrunner_instance)))

(fn SetWaitforTiles
  (params (SetWaitForTiles :type Integer))
  (bind _asrunner_instance (Utilities|Casting|CastToRunnerInstance (Game|GetGameInstance)))
  (Variables|/Game/Assets/Blueprints/RunnerInstance.RunnerInstance_C|SetWaitForTiles _asrunner_instance SetWaitForTiles))